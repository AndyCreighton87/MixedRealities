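; BP_StaticBodyPart cycles one static-mesh body part on a character model, as part of the character creator.
; Next and previous events step an index through the BodyParts mesh array, then call UpdateBodyPart.
; UpdateBodyPart finds the model's first StaticMeshComponent with the configured Tag and assigns the selected mesh.
; The increment wraps by array length, while the decrement takes its modulo against index plus length.
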(event `/Game/6106MixedRealities/Blueprints/Interfaces/IBodyPartData.NextBodyPart`
  (params (Model :type "/Game/6106MixedRealities/Blueprints/Characters/BP_BaseConcertCharacter Object Reference"))
  (`self.IncrementIndex`)
  (`/Game/6106MixedRealities/Blueprints/Interfaces/IBodyPartData.UpdateBodyPart` Model))

(event `/Game/6106MixedRealities/Blueprints/Interfaces/IBodyPartData.PrevBodyPart`
  (params (Model :type "/Game/6106MixedRealities/Blueprints/Characters/BP_BaseConcertCharacter Object Reference"))
  (`self.DecrementIndex`)
  (`/Game/6106MixedRealities/Blueprints/Interfaces/IBodyPartData.UpdateBodyPart` Model))

(event `/Game/6106MixedRealities/Blueprints/Interfaces/IBodyPartData.UpdateBodyPart`
  (params (Model :type "/Game/6106MixedRealities/Blueprints/Characters/BP_BaseConcertCharacter Object Reference"))
  (`StaticMeshComponent.SetStaticMesh` (`|GetArrayItem` (`self.GetComponentsByTag` Model "/Script/Engine.StaticMeshComponent" (`self.Tag`))) (`|GetArrayItem` (`self.BodyParts`) (`self.Index`))))

(fn `DecrementIndex`
  (bind _returnvalue (+ (`self.Index`) (`KismetArrayLibrary.Array_Length` (`self.BodyParts`))))
  (bind _result (`/Engine/EditorBlueprintResources/StandardMacros.DecrementInt` _returnvalue)
    (:`  `
      (set `self.Index` (mod _result _returnvalue)))))

(fn `IncrementIndex`
  (bind _result (`/Engine/EditorBlueprintResources/StandardMacros.IncrementInt` (`self.Index`))
    (:`  `
      (set `self.Index` (mod _result (`KismetArrayLibrary.Array_Length` (`self.BodyParts`)))))))

(fn `UserConstructionScript`)