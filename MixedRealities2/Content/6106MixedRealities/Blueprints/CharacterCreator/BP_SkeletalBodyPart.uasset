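; Character creator Blueprint that cycles one body part of a model through an array of skeletal meshes.
; Next and previous events step an index with modulo wraparound in both directions, then trigger an update on the given model.
; The update finds the model's first skeletal mesh component with the configured tag and sets its mesh to the selected entry, reinitializing the pose.
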(event `self.NextBodyPart`
  (params (Model :type "/Game/6106MixedRealities/Blueprints/Characters/BP_BaseConcertCharacter Object Reference"))
  (`self.IncrementIndex`)
  (`self.UpdateBodyPart` Model))

(event `self.PrevBodyPart`
  (params (Model :type "/Game/6106MixedRealities/Blueprints/Characters/BP_BaseConcertCharacter Object Reference"))
  (`self.DecrementIndex`)
  (`self.UpdateBodyPart` Model))

(event `self.UpdateBodyPart`
  (params (Model :type "/Game/6106MixedRealities/Blueprints/Characters/BP_BaseConcertCharacter Object Reference"))
  (`SkinnedMeshComponent.SetSkinnedAssetAndUpdate` (`|GetArrayItem` (`self.GetComponentsByTag` Model "/Script/Engine.SkeletalMeshComponent" (`self.Tag`))) (`|GetArrayItem` (`self.BodyParts`) (`self.Index`)) true))

(fn `DecrementIndex`
  (bind _returnvalue (`KismetArrayLibrary.Array_Length` (`self.BodyParts`)))
  (bind _result (`/Engine/EditorBlueprintResources/StandardMacros.DecrementInt` (+ (`self.Index`) _returnvalue))
    (:`  `
      (set `self.Index` (mod _result _returnvalue)))))

(fn `IncrementIndex`
  (bind _result (`/Engine/EditorBlueprintResources/StandardMacros.IncrementInt` (`self.Index`))
    (:`  `
      (set `self.Index` (mod _result (`KismetArrayLibrary.Array_Length` (`self.BodyParts`)))))))

(fn `UserConstructionScript`)