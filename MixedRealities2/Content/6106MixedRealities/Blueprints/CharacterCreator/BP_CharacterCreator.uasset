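; Character creator actor that manages swappable head, chest, legs, hands and hair parts for a Model.
; On BeginPlay it spawns one body part actor per slot at its own root transform and stores each.
; Next and previous functions delegate cycling to the given part, passing it the Model.
; A helper returns the Model's skeletal meshes and static hair mesh by tag lookup, though every tag is None.
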(event `self.ReceiveBeginPlay`
  (`self.InitializeBodyParts`))

(fn `GetMeshComponents`
  (returns (Chest :type "SkeletalMeshComponent Object Reference") (Head :type "SkeletalMeshComponent Object Reference") (Legs :type "SkeletalMeshComponent Object Reference") (Hands :type "SkeletalMeshComponent Object Reference") (Hair :type "StaticMeshComponent Object Reference"))
  (bind _model (`self.Model`))
  ;[1 1 1] Get Components
  (return (`|GetArrayItem` (`self.GetComponentsByTag` _model "/Script/Engine.SkeletalMeshComponent" "None")) (`|GetArrayItem` (`self.GetComponentsByTag` _model "/Script/Engine.SkeletalMeshComponent" "None")) (`|GetArrayItem` (`self.GetComponentsByTag` _model "/Script/Engine.SkeletalMeshComponent" "None")) (`|GetArrayItem` (`self.GetComponentsByTag` _model "/Script/Engine.SkeletalMeshComponent" "None")) (`|GetArrayItem` (`self.GetComponentsByTag` _model "/Script/Engine.StaticMeshComponent" "None"))))

(fn `InitializeBodyParts`
  (bind _returnvalue (`SceneComponent.K2_GetComponentToWorld` (`self.DefaultSceneRoot`)))
  (bind _returnvalue_2 (`|SpawnActorFromClass` "/Game/6106MixedRealities/Blueprints/CharacterCreator/BodyParts/BP_HeadBodyPart.BP_HeadBodyPart_C" _returnvalue "Undefined" "OverrideRootScale" null null))
  (set `self.Head` _returnvalue_2)
  (bind _returnvalue_3 (`|SpawnActorFromClass` "/Game/6106MixedRealities/Blueprints/CharacterCreator/BodyParts/BP_ChestBodyPart.BP_ChestBodyPart_C" _returnvalue "Undefined" "OverrideRootScale" null null))
  (set `self.Chest` _returnvalue_3)
  (bind _returnvalue_4 (`|SpawnActorFromClass` "/Game/6106MixedRealities/Blueprints/CharacterCreator/BodyParts/BP_LegsBodyPart.BP_LegsBodyPart_C" _returnvalue "Undefined" "OverrideRootScale" null null))
  (set `self.Legs` _returnvalue_4)
  (bind _returnvalue_5 (`|SpawnActorFromClass` "/Game/6106MixedRealities/Blueprints/CharacterCreator/BodyParts/BP_HandsBodyPart.BP_HandsBodyPart_C" _returnvalue "Undefined" "OverrideRootScale" null null))
  (set `self.Hands` _returnvalue_5)
  (bind _returnvalue_6 (`|SpawnActorFromClass` "/Game/6106MixedRealities/Blueprints/CharacterCreator/BodyParts/BP_HairBodyPart.BP_HairBodyPart_C" _returnvalue "Undefined" "OverrideRootScale" null null))
  (set `self.Hair` _returnvalue_6))

(fn `NextBodyPart`
  (params (BodyPart :type "/Game/6106MixedRealities/Blueprints/Interfaces/IBodyPartData Interface"))
  (`/Game/6106MixedRealities/Blueprints/Interfaces/IBodyPartData.NextBodyPart` BodyPart (`self.Model`)))

(fn `PrevBodyPart`
  (params (BodyPart :type "/Game/6106MixedRealities/Blueprints/Interfaces/IBodyPartData Interface"))
  (`/Game/6106MixedRealities/Blueprints/Interfaces/IBodyPartData.PrevBodyPart` BodyPart (`self.Model`)))

(fn `UserConstructionScript`)