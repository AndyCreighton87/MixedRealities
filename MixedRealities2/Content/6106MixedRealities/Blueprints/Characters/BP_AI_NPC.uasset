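; BP_AI_NPC is an NPC character that spawns an emoji generator and can show a person profile widget.
; On BeginPlay it attaches a new EmojiGenerator at EmojiSpawnPoint.
; Focus events toggle custom depth on the body-part meshes for highlighting, and both hide any open profile.
; ManageUI toggles the profile, creating the widget on demand and filling it from PersonInfo whenever shown.
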(event `self.ReceiveBeginPlay`
  ;[1 1 1] Emoji Spawning
  (bind _returnvalue (`|SpawnActorFromClass` "/Game/6106MixedRealities/Blueprints/Emotes/EmojiGenerator.EmojiGenerator_C" (`KismetMathLibrary.MakeTransform` (0.0 0.0 0.0)) "Undefined" "OverrideRootScale" null null))
  (`self.K2_AttachToComponent` _returnvalue (`self.EmojiSpawnPoint`) "None" "SnapToTarget" "KeepRelative" "KeepRelative" false))

(event `AddWidget`
  (bind _personprofilewidget (`self.PersonProfileWidget`))
  ;[1 1 1] Adds Person Profile to Viewport & Updates UI Data
  (`UserWidget.AddToViewport` _personprofilewidget 0)
  (`/Game/6106MixedRealities/Blueprints/Widgets/Widget_PersonProfile.UpdateUIData` _personprofilewidget (`self.PersonInfo`))
  (set `self.IsWidgetActive` true))

(event `RemoveWidget`
  ;[1 1 1] Removes Person Profile from Viewport
  (`Widget.RemoveFromParent` (`self.PersonProfileWidget`))
  (set `self.IsWidgetActive` false))

(fn `CreateNewWidget`
  ;[1 1 1] Creates a new Person Profile Widget
  (bind _returnvalue (`|CreateWidget` "/Game/6106MixedRealities/Blueprints/Widgets/Widget_PersonProfile.Widget_PersonProfile_C" (`GameplayStatics.GetPlayerController` 0)))
  (set `self.PersonProfileWidget` _returnvalue))

(fn `HideUI`
  ;[1 1 1] Hide UI
  (if (`self.IsWidgetActive`)
    (`self.RemoveWidget`)))

(fn `ManageUI`
  ;[1 1 1] Manage Display of Person Profile
  (if (`self.IsWidgetActive`)
    (`self.RemoveWidget`)
    (else
      (if (not (`KismetSystemLibrary.IsValid` (`self.PersonProfileWidget`)))
        (`self.CreateNewWidget`))
      (`self.AddWidget`))))

(fn `OnFocus`
  ;[1 1 1] Add highlight to mesh
  (`PrimitiveComponent.SetRenderCustomDepth` (`self.Mesh`) true)
  (`PrimitiveComponent.SetRenderCustomDepth` (`self.Hands`) true)
  (`PrimitiveComponent.SetRenderCustomDepth` (`self.Legs`) true)
  (`PrimitiveComponent.SetRenderCustomDepth` (`self.Head`) true)
  (`PrimitiveComponent.SetRenderCustomDepth` (`self.Hair`) true)
  (`PrimitiveComponent.SetRenderCustomDepth` (`self.Eyes`) true)
  (`self.HideUI`))

(fn `OnFocusEnd`
  ;[1 1 1] Remove highlight from mesh
  (`PrimitiveComponent.SetRenderCustomDepth` (`self.Mesh`) false)
  (`PrimitiveComponent.SetRenderCustomDepth` (`self.Hands`) false)
  (`PrimitiveComponent.SetRenderCustomDepth` (`self.Legs`) false)
  (`PrimitiveComponent.SetRenderCustomDepth` (`self.Head`) false)
  (`PrimitiveComponent.SetRenderCustomDepth` (`self.Hair`) false)
  (`PrimitiveComponent.SetRenderCustomDepth` (`self.Eyes`) false)
  (`self.HideUI`))

(fn `UserConstructionScript`
  (`parent.UserConstructionScript`))