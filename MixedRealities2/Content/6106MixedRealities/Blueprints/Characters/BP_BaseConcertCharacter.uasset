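; BP_BaseConcertCharacter is a base Blueprint for modular concert characters with an attached emoji generator.
; The construction script makes Head, Hands and Legs follow the main Mesh through master pose, and snaps Eyes and Hair to its headSocket.
; On BeginPlay it spawns an EmojiGenerator actor, stores the reference and attaches it to EmojiSpawnPoint.
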(event `self.ReceiveBeginPlay`
  ;[1 1 1] Create EmojiGenerator
  (bind _returnvalue (`|SpawnActorFromClass` "/Game/6106MixedRealities/Blueprints/Emotes/EmojiGenerator.EmojiGenerator_C" (`KismetMathLibrary.MakeTransform` (0.0 0.0 0.0)) "Undefined" "OverrideRootScale" null null))
  (bind _output_get (set `self.EmojiGenerator` _returnvalue))
  (`self.K2_AttachToComponent` _output_get (`self.EmojiSpawnPoint`) "None" "SnapToTarget" "KeepRelative" "KeepRelative" true))

(fn `UserConstructionScript`
  (`SkinnedMeshComponent.SetLeaderPoseComponent` (`self.Head`) (`self.Mesh`) false)
  (`SkinnedMeshComponent.SetLeaderPoseComponent` (`self.Hands`) (`self.Mesh`) false)
  (`SkinnedMeshComponent.SetLeaderPoseComponent` (`self.Legs`) (`self.Mesh`) false)
  (`SceneComponent.K2_AttachToComponent` (`self.Eyes`) (`self.Mesh`) "headSocket" "SnapToTarget" "SnapToTarget" "KeepRelative" true)
  (`SceneComponent.K2_AttachToComponent` (`self.Hair`) (`self.Mesh`) "headSocket" "SnapToTarget" "SnapToTarget" "KeepRelative" true))