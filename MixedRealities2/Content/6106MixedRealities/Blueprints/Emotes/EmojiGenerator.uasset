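; Emote emoji spawner that periodically creates Emoji actors while an emote is active.
; StartSpawning stores the emote and enables a looping timer event, which stops spawning once accumulated intervals reach the emote lifetime or EndSpawning is called.
; Spawn location derives from a spawn-point component through random-offset helpers, whose offset math appears unconnected.
; The widget setup call never runs, so the stored emote does not affect spawned emojis here.
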(event `self.ReceiveBeginPlay`
  ;[1 1 1] Set Emoji Spawning Event
  (`KismetSystemLibrary.K2_SetTimerDelegate` (delegate `SpawnEmojis`) (`self.EmojiSpawnTimer`) true))

(event `SpawnEmojis`
  ;[1 1 1] Set Emoji Spawning Event
  (if (`self.CanSpawn`)
    (`self.CreateNewEmoji`)
    (`self.EmojiTimer` (`self.EmojiSpawnTimer`))))

(fn `CreateNewEmoji`
  (`|SpawnActorFromClass` "/Game/6106MixedRealities/Blueprints/Emotes/Emoji.Emoji_C" (`KismetMathLibrary.MakeTransform` (`self.GetEmojiSpawnLocation`)) "Undefined" "OverrideRootScale" null null))

(fn `EmojiTimer`
  (params (Time :type "Float (double-precision)"))
  ;[1 1 1] Manage LifeTime of Emote
  (bind _output_get (set `self.EmoteElaspedTime` (+ Time (`self.EmoteElaspedTime`))))
  (if (>= _output_get (`self.EmoteLifetime`))
    (set `self.CanSpawn` false)
    (set `self.EmoteElaspedTime` 0.0)))

(fn `EndSpawning`
  ;[1 1 1] End Spawning
  (set `self.CurrentEmote` (struct))
  (set `self.CanSpawn` false))

(fn `GetEmojiSpawnLocation`
  (returns (Pos :type "Vector Structure"))
  (bind (_returnvalue_x _returnvalue_y _returnvalue_z) (`KismetMathLibrary.BreakVector` (`SceneComponent.K2_GetComponentLocation` (`self.EmojiSpawnPoint`))))
  ;[1 1 1] Gets Randomised Spawn Point
  (return (`KismetMathLibrary.MakeVector` (`self.EmojiSpawningRandomValue` _returnvalue_x) (`self.EmojiSpawningRandomValueBothSides` _returnvalue_y) (`self.EmojiSpawningRandomValue` _returnvalue_z))))

(fn `StartSpawning`
  (params (NewParam :type "/Game/6106MixedRealities/Blueprints/Structs/Struct_Emotes Structure"))
  ;[1 1 1] Start Spawning
  (set `self.CurrentEmote` NewParam)
  (set `self.CanSpawn` true))

(fn `UserConstructionScript`)