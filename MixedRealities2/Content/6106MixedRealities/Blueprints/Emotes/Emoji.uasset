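; Floating emote actor that carries a widget upward and destroys itself once its lifetime runs out.
; Each tick it rises on Z at a speed randomized every frame between Speed and Speed times SpeedVariance.
; The widget turns toward the player pawn's location, rather than the camera, with pitch locked at zero.
; RandomizeSize runs each tick but does nothing, as its scaling nodes are disconnected.
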(event `self.ReceiveTick`
  (params (DeltaSeconds :type "Float (single-precision)"))
  (`self.MoveUpwards` DeltaSeconds)
  (`self.LookAtCamera`)
  (`self.ManageLifetime` DeltaSeconds)
  (`self.RandomizeSize`))

(fn `Destroy`
  (set `self.HasExpired` true)
  (`self.K2_DestroyActor`))

(fn `LookAtCamera`
  ;[1 1 1] Widget will always face the camera on X and Z axis
  (`SceneComponent.K2_SetWorldRotation` (`self.Widget`) (`KismetMathLibrary.MakeRotator` (.roll (`KismetMathLibrary.FindLookAtRotation` (`self.K2_GetActorLocation` (`GameplayStatics.GetPlayerPawn` 0)) (`SceneComponent.K2_GetComponentLocation` (`self.Widget`)))) 0.0 (+ (.yaw (`KismetMathLibrary.FindLookAtRotation` (`self.K2_GetActorLocation` (`GameplayStatics.GetPlayerPawn` 0)) (`SceneComponent.K2_GetComponentLocation` (`self.Widget`)))) 180.0)) false false))

(fn `ManageLifetime`
  (params (DeltaTime :type "Float (double-precision)"))
  ;[1 1 1] If the Lifetime has elapsed, Destroy self
  (if (not (`self.HasExpired`))
    (bind _output_get (set `self.ElapsedTime` (+ DeltaTime (`self.ElapsedTime`))))
    (if (>= _output_get (`self.LifeTime`))
      (`self.Destroy`))))

(fn `MoveUpwards`
  (params (DeltaTime :type "Float (double-precision)"))
  ;[1 1 1] Moves Widget Upwards on Z axis
  (`self.K2_SetActorLocation` (+ (`KismetMathLibrary.MakeVector` 0.0 0.0 (* DeltaTime (`KismetMathLibrary.RandomFloatInRange` (`self.Speed`) (* (`self.Speed`) (`self.SpeedVariance`))))) (`self.K2_GetActorLocation`))))

(fn `RandomizeSize`)

(fn `UserConstructionScript`)