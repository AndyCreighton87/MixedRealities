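; BP_CharacterCreator swaps modular body part meshes on a Model to build a customizable character.
; Next and Prev functions step a body part's index with modulo wraparound through its mesh pool, apply it and return the updated data struct.
; Update functions find the target component by tag, with separate skeletal and static mesh variants.
; GetMeshComponents returns the tagged chest, hands, legs and head skeletal components and the static hair component.
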(fn `GetMeshComponents`
  (returns (Chest :type "SkeletalMeshComponent Object Reference") (Hands :type "SkeletalMeshComponent Object Reference") (Legs :type "SkeletalMeshComponent Object Reference") (Head :type "SkeletalMeshComponent Object Reference") (Hair :type "StaticMeshComponent Object Reference"))
  (return (`|GetArrayItem` (`self.GetComponentsByTag` (`self.Model`) "/Script/Engine.SkeletalMeshComponent" "Chest")) (`|GetArrayItem` (`self.GetComponentsByTag` (`self.Model`) "/Script/Engine.SkeletalMeshComponent" "Hands")) (`|GetArrayItem` (`self.GetComponentsByTag` (`self.Model`) "/Script/Engine.SkeletalMeshComponent" "Legs")) (`|GetArrayItem` (`self.GetComponentsByTag` (`self.Model`) "/Script/Engine.SkeletalMeshComponent" "Head")) (`|GetArrayItem` (`self.GetComponentsByTag` (`self.Model`) "/Script/Engine.StaticMeshComponent" "Hair"))))

(fn `NextBodypartSkeletal`
  (params (BodypartData :type "/Game/MixedRealityAssignment/Structs/BodyPartSkeletalData_Struct Structure"))
  (returns (BodyPartStruct :type "/Game/MixedRealityAssignment/Structs/BodyPartSkeletalData_Struct Structure"))
  (locals (BodyapartLocal :type "/Game/MixedRealityAssignment/Structs/BodyPartSkeletalData_Struct Structure"))
  (bind (_tag _bodypartpool _index) (break `/Game/MixedRealityAssignment/Structs/BodyPartSkeletalData_Struct` BodypartData))
  ;[1 1 1] Next Bodaypart
  (bind _result (`/Engine/EditorBlueprintResources/StandardMacros.IncrementInt` _index)
    (:`  `
      (bind _bodypartskeletaldata_struct (make `/Game/MixedRealityAssignment/Structs/BodyPartSkeletalData_Struct` _tag _bodypartpool (mod _result (`KismetArrayLibrary.Array_Length` _bodypartpool))))
      (`self.UpdateBodypartSkeletal` _bodypartskeletaldata_struct)
      (return _bodypartskeletaldata_struct))))

(fn `NextBodypartStatic`
  (params (BodypartData :type "/Game/MixedRealityAssignment/Structs/BodyPartStaticData_Struct Structure"))
  (returns (NewParam :type "/Game/MixedRealityAssignment/Structs/BodyPartStaticData_Struct Structure"))
  (locals (LocalBodyPart :type "/Game/MixedRealityAssignment/Structs/BodyPartStaticData_Struct Structure"))
  (bind (_tag _bodypartpool _index) (break `/Game/MixedRealityAssignment/Structs/BodyPartStaticData_Struct` BodypartData))
  ;[1 1 1] Next Bodypart
  (bind _result (`/Engine/EditorBlueprintResources/StandardMacros.IncrementInt` _index)
    (:`  `
      (bind _bodypartstaticdata_struct (make `/Game/MixedRealityAssignment/Structs/BodyPartStaticData_Struct` _tag _bodypartpool (mod _result (`KismetArrayLibrary.Array_Length` _bodypartpool))))
      (`self.UpdateBodypartStatic` _bodypartstaticdata_struct)
      (return _bodypartstaticdata_struct))))

(fn `PrevBodypartSkeletal`
  (params (BodypartData :type "/Game/MixedRealityAssignment/Structs/BodyPartSkeletalData_Struct Structure"))
  (returns (BodyPartStruct :type "/Game/MixedRealityAssignment/Structs/BodyPartSkeletalData_Struct Structure"))
  (locals (BodypartLocal :type "/Game/MixedRealityAssignment/Structs/BodyPartSkeletalData_Struct Structure"))
  (bind (_tag _bodypartpool _index) (break `/Game/MixedRealityAssignment/Structs/BodyPartSkeletalData_Struct` BodypartData))
  (bind _returnvalue (`KismetArrayLibrary.Array_Length` _bodypartpool))
  ;[1 1 1] Prev Bodypart
  (bind _result (`/Engine/EditorBlueprintResources/StandardMacros.DecrementInt` (+ _returnvalue _index))
    (:`  `
      (bind _bodypartskeletaldata_struct (make `/Game/MixedRealityAssignment/Structs/BodyPartSkeletalData_Struct` _tag _bodypartpool (mod _result _returnvalue)))
      (`self.UpdateBodypartSkeletal` _bodypartskeletaldata_struct)
      (return _bodypartskeletaldata_struct))))

(fn `PrevBodypartStatic`
  (params (BodypartData :type "/Game/MixedRealityAssignment/Structs/BodyPartStaticData_Struct Structure"))
  (returns (BodyPartStruct :type "/Game/MixedRealityAssignment/Structs/BodyPartStaticData_Struct Structure"))
  (locals (BodyPartLocal :type "/Game/MixedRealityAssignment/Structs/BodyPartStaticData_Struct Structure"))
  (bind (_tag _bodypartpool _index) (break `/Game/MixedRealityAssignment/Structs/BodyPartStaticData_Struct` BodypartData))
  (bind _returnvalue (`KismetArrayLibrary.Array_Length` _bodypartpool))
  ;[1 1 1] Prev Bodypart
  (bind _result (`/Engine/EditorBlueprintResources/StandardMacros.DecrementInt` (+ _returnvalue _index))
    (:`  `
      (bind _bodypartstaticdata_struct (make `/Game/MixedRealityAssignment/Structs/BodyPartStaticData_Struct` _tag _bodypartpool (mod _result _returnvalue)))
      (`self.UpdateBodypartStatic` _bodypartstaticdata_struct)
      (return _bodypartstaticdata_struct))))

(fn `UpdateBodypartSkeletal`
  (params (`Bodypart Data` :type "/Game/MixedRealityAssignment/Structs/BodyPartSkeletalData_Struct Structure"))
  ;[1 1 1] Set Bodypart
  (`SkinnedMeshComponent.SetSkinnedAssetAndUpdate` (`|GetArrayItem` (`self.GetComponentsByTag` (`self.Model`) "/Script/Engine.SkeletalMeshComponent" `Bodypart Data_Tag_12_04794C7D4A935A479FC40EA2B88B7704`)) (`|GetArrayItem` `Bodypart Data_BodypartPool_7_E2E8BFFB4D30D4C4C34125A7C3F42F3B` `Bodypart Data_Index_5_6422628B4DDFBBADD12A89AE43293897`) false))

(fn `UpdateBodypartStatic`
  (params (`Bodypart Data` :type "/Game/MixedRealityAssignment/Structs/BodyPartStaticData_Struct Structure"))
  ;[1 1 1] Set Bodypart
  (`StaticMeshComponent.SetStaticMesh` (`|GetArrayItem` (`self.GetComponentsByTag` (`self.Model`) "/Script/Engine.StaticMeshComponent" `Bodypart Data_Tag_11_E2E8BFFB4D30D4C4C34125A7C3F42F3B`)) (`|GetArrayItem` `Bodypart Data_BodypartPool_10_D01691714A7317FE4B6DD68EC77B2AB1` `Bodypart Data_Index_9_1DC3B7A64E9C14080EF7E99E47015A0B`)))

(fn `UserConstructionScript`)