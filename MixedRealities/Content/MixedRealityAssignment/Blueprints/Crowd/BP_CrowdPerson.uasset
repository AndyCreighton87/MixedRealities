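; BP_CrowdPerson is a modular crowd character that highlights on focus through custom depth and has a profile widget.
; Construction makes head, hands and legs follow the body mesh's pose and snaps eyes and hair to its head socket.
; ManageUI lazily creates the widget and fills it from PersonInfo.
; Toggle-off and focus-loss hiding depend on IsWidgetActive, whose set-to-true node is unwired.
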(event `AddWidget`
  (bind _personprofilewidget (`self.PersonProfileWidget`))
  ;[1 1 1] Adds Person Profile to Viewport & Update UI Data
  (`UserWidget.AddToViewport` _personprofilewidget 0)
  (`/Game/MixedRealityAssignment/Widgets/Widget_PersonProfile.UpdateUIData` _personprofilewidget (`self.PersonInfo`)))

(event `RemoveWidget`
  ;[1 1 1] Removes Person Profile from Viewport
  (`Widget.RemoveFromParent` (`self.PersonProfileWidget`))
  (set `self.IsWidgetActive` false))

(fn `CreateNewWidget`
  ;[1 1 1] Creates a new Profile Widget
  (bind _returnvalue (`|CreateWidget` "/Game/MixedRealityAssignment/Widgets/Widget_PersonProfile.Widget_PersonProfile_C" (`GameplayStatics.GetPlayerController` 0)))
  (set `self.PersonProfileWidget` _returnvalue))

(fn `HideUI`
  (if (`self.IsWidgetActive`)
    (`self.RemoveWidget`)))

(fn `ManageUI`
  ;[1 1 1] Manage Display of User Profile
  (if (`self.IsWidgetActive`)
    (`self.RemoveWidget`)
    (else
      (if (not (`KismetSystemLibrary.IsValid` (`self.PersonProfileWidget`)))
        (`self.CreateNewWidget`))
      (`self.AddWidget`))))

(fn `OnEndFocus`
  (`PrimitiveComponent.SetRenderCustomDepth` (`self.Mesh`) false)
  (`self.HideUI`))

(fn `OnFocus`
  (`PrimitiveComponent.SetRenderCustomDepth` (`self.Mesh`) true))

(fn `UserConstructionScript`
  (`SkinnedMeshComponent.SetLeaderPoseComponent` (`self.Head`) (`self.Mesh`) false)
  (`SkinnedMeshComponent.SetLeaderPoseComponent` (`self.Hands`) (`self.Mesh`) false)
  (`SkinnedMeshComponent.SetLeaderPoseComponent` (`self.Legs`) (`self.Mesh`) false)
  (`SceneComponent.K2_AttachToComponent` (`self.Eyes`) (`self.Mesh`) "headSocket" "SnapToTarget" "SnapToTarget" "KeepRelative" true)
  (`SceneComponent.K2_AttachToComponent` (`self.Hair`) (`self.Mesh`) "headSocket" "SnapToTarget" "SnapToTarget" "KeepRelative" true))